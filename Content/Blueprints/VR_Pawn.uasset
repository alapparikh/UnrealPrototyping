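; VR pawn that tracks where the headset sits within the SteamVR play area.
; On BeginPlay it sets a floor tracking origin and starts a one-second looping timer.
; Each timer call divides the camera's world XY by the first chaperone bound, then ModifyFloatRange clamps and remaps each axis to 0–1 in NormalizedPos.
; Tick is empty, and the debug print chains are disconnected.
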(event `self.ReceiveBeginPlay`
  (`HeadMountedDisplayFunctionLibrary.SetTrackingOrigin` "Floor")
  (`KismetSystemLibrary.K2_SetTimerDelegate` (delegate `Bounds data`) 1.0 true))

(event `Bounds data`
  (bind (_returnvalue_x _returnvalue_y) (`KismetMathLibrary.BreakVector` (/ (* (`SceneComponent.K2_GetComponentLocation` (`self.VRCamera`)) (1.0 1.0 0.0)) (+ (`|GetArrayItem` (`SteamVRChaperoneComponent.GetBounds` (`self.SteamVRChaperone`))) (0.0 0.0 1.0)))))
  (bind _outputfloat (`self.ModifyFloatRange` _returnvalue_x))
  (bind _outputfloat_2 (`self.ModifyFloatRange` _returnvalue_y))
  (bind _output_get (set `self.NormalizedPos` (`KismetMathLibrary.MakeVector` _outputfloat _outputfloat_2))))

(event `self.ReceiveTick`
  (params (DeltaSeconds :type "Float (single-precision)")))

(fn `ModifyFloatRange`
  (params (InputFloat :type "Float (double-precision)"))
  (returns (OutputFloat :type "Float (double-precision)"))
  (return (/ (+ (`KismetMathLibrary.FClamp` InputFloat -1.0) 1.0) 2.0)))

(fn `UserConstructionScript`)